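; Base Blueprint for a game device with a state machine covering working, attached, hacked, power-surge shorted and destroyed states.
; UpdateDeviceState sets the state, fires cosmetic events for hacking and destruction, and has MyGameMode check win conditions on destruction.
; Power surge functions short working or attached devices and restore shorted ones, depending on current state.
; Cosmetic and server-named events are empty hooks, including the one attachment updates forward to.
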(event Custom|SetDeviceState
  (params (NewState :type DeviceState%20Enum))
  (Variables|Default|SetDeviceState NewState))

(event Custom|BeginPowerSurgeServer)

(event Custom|UpdateDeviceStateServer
  (params (New%20State :type DeviceState%20Enum)))

(event Custom|EndPowerSurgeServer)

(event Custom|DeathEventCosmetic)

(event Custom|BeingHackedCosmetic)

(event Custom|UpdateAttachmentServer
  (params (ActorCalled :type Actor%20Object%20Reference)))

(event EventUpdateDeviceState
  (params (NewState :type DeviceState%20Enum :default "NewEnumerator0"))
  (CallFunction|SetDeviceState NewState)
  (switch Utilities|FlowControl|Switch|SwitchonDeviceState NewState
    (:NewEnumerator1
      (CallFunction|BeingHackedCosmetic))
    (:NewEnumerator2
      (bind _asmy_game_mode (Utilities|Casting|CastToMyGameMode (Game|GetGameMode)))
      (Default|CheckWinConditions _asmy_game_mode)
      (CallFunction|DeathEventCosmetic))))

(event EventBeginPlay)

(event EventActorBeginOverlap
  (params (OtherActor :type Actor%20Object%20Reference)))

(event EventTick
  (params (DeltaSeconds :type Float%20%28single-precision%29)))

(event EventUpdateAttachment
  (params (Actor :type Actor%20Object%20Reference))
  (CallFunction|UpdateAttachmentServer Actor))

(fn ConstructionScript)

(fn PowerSurgeStart
  (switch Utilities|FlowControl|Switch|SwitchonDeviceState (Variables|Default|GetDeviceState)
    (:NewEnumerator0
      _)
    (:NewEnumerator4
      _))
  ;[1 1 1] Doing Attached, Cause button may be in process of detaching
  (CallFunction|BeginPowerSurgeServer)
  (CallFunction|UpdateDeviceState "NewEnumerator3"))

(fn PowerSurgeEnd
  (switch Utilities|FlowControl|Switch|SwitchonDeviceState (Variables|Default|GetDeviceState)
    (:NewEnumerator4
      ;[1 1 1] Button may already be attached
      (CallFunction|EndPowerSurgeServer))
    (:NewEnumerator3
      (CallFunction|EndPowerSurgeServer)
      (CallFunction|UpdateDeviceState "NewEnumerator0"))))