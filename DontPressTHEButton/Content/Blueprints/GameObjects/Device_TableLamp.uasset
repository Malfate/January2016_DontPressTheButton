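; Table lamp device that players can switch on and off and that can be destroyed.
; Interaction toggles the point light while the device is Working or Being Hacked, and the light component's replication is disabled at BeginPlay.
; Destruction sets the Destroyed state and turns the light off, with a separate cosmetic event for hit particles and sound.
; An attachment toggle hides or shows the mesh by flipping IsAttachedTo.
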(event Custom|TurnOffLight
  (Rendering|SetVisibility (Variables|Default|GetPointLight) false false))

(event Custom|ToggleLight
  (Rendering|ToggleVisibility (Variables|Default|GetPointLight) false))

(event EventToggleAttachment
  (params (Actor :type Actor%20Object%20Reference))
  (bind _staticmesh1 (Variables|Default|GetStaticMesh1))
  (if (Variables|Default|GetbIsAttachedTo)
    (Development|SetHiddeninGame _staticmesh1 false false)
    (Variables|Default|SetbIsAttachedTo false)
    (else
      (Development|SetHiddeninGame _staticmesh1 true false)
      (Variables|Default|SetbIsAttachedTo true))))

(event EventDeathEventCosmetic
  (bind _staticmesh1 (Variables|Default|GetStaticMesh1))
  (bind _returnvalue (Transformation|GetWorldLocation _staticmesh1))
  (Effects|SpawnEmitteratLocation "/Game/Effects/P_Hit.P_Hit" _returnvalue)
  (Audio|PlaySoundatLocation "/Game/Sounds/Laser_01.Laser_01" _returnvalue))

(event EventDestroyObject
  (params (Actor :type Actor%20Object%20Reference))
  (CallFunction|UpdateDeviceState "NewEnumerator2")
  (CallFunction|TurnOffLight))

(event EventBeginPlay
  (Class|ActorComponent|SetIsReplicated (Variables|Default|GetPointLight) false))

(event EventActorBeginOverlap
  (params (OtherActor :type Actor%20Object%20Reference)))

(event EventTick
  (params (DeltaSeconds :type Float%20%28single-precision%29)))

(event EventInteractwithObject
  (params (InteractingActor :type Actor%20Object%20Reference))
  (switch Utilities|FlowControl|Switch|SwitchonDeviceState (Variables|Default|GetDeviceState)
    (:NewEnumerator0
      _)
    (:NewEnumerator1
      _))
  (CallFunction|ToggleLight))

(fn ConstructionScript
  (|CallParentFunction))